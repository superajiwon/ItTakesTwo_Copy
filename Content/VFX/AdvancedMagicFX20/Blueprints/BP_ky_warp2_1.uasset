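; BP_ky_warp2_1 is a timed warp particle effect actor with a configurable color and duration, optionally looping.
; BeginPlay activates the FX component and drives its size through start and end timelines, then fades dust, deactivates, and either restarts or destroys the actor.
; Tick counts Duration down, cutting core spawning near the end and spawning a tinted P_ky_warpEnd burst once.
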(event `self.ReceiveBeginPlay`
  (bind _fx (`self.FX`))
  (bind _duration (`self.duration`))
  ;[1 1 1] particle enable
  (`ParticleSystemComponent.SetFloatParameter` _fx "dust" 700.0 :!label _label)
  (`ParticleSystemComponent.SetFloatParameter` _fx "core" 5.0)
  ;[1 1 1] set duration
  (`ParticleSystemComponent.SetFloatParameter` _fx "life" _duration)
  (set `self.durationTmp` _duration)
  ;[1 1 1] effect on
  (`ActorComponent.Activate` (`self.FX`) false)
  ;[1 1 1] size control 1st
  (bind (_direction _newtrack_0) (`Timeline|Timeline_sizeStart` :!via `PlayFromStart`)
    (:`Update`
      (`ParticleSystemComponent.SetVectorParameter` (`self.FX`) "size" (`KismetMathLibrary.Conv_DoubleToVector` _newtrack_0))
      ;[1 1 1] loop control
      (if (> (`self.duration`) 0.7) :!label _label_2
        (`KismetSystemLibrary.Delay` 0.05)
        (goto _label_2)
        (else
          ;[1 1 1] size control 2nd
          (bind (_direction_2 _newtrack_0_2 _newtrack_2) (`Timeline|Timeline_sizeEnd` :!via `PlayFromStart`)
            (:`Update`
              (`ParticleSystemComponent.SetVectorParameter` (`self.FX`) "size" (`KismetMathLibrary.Conv_DoubleToVector` _newtrack_0_2))
              (`ParticleSystemComponent.SetVectorParameter` (`self.FX`) "ringSize" _newtrack_2)
              ;[1 1 1] dust particle off
              (`KismetSystemLibrary.Delay` 0.5)
              (`ParticleSystemComponent.SetFloatParameter` (`self.FX`) "dust" 0.0)
              (`KismetSystemLibrary.Delay` 0.2)
              ;[1 1 1] effect off
              (`ActorComponent.Deactivate` (`self.FX`))
              (`KismetSystemLibrary.Delay` 2.0)
              ;[1 1 1] determine whether to repeat,
              ; if true - repeat , if false - destroy
              (if (`self.isLoop`)
                ;[1 1 1] init
                (set `self.duration` (`self.durationTmp`))
                (set `self.isEnd` false)
                (goto _label)
                (else
                  ;[1 1 1] effect destroy
                  (`self.K2_DestroyActor`))))))))))

(event `self.ReceiveTick`
  (params (DeltaSeconds :type "Float (single-precision)"))
  (bind _defaultsceneroot (`self.DefaultSceneRoot`))
  ;[1 1 1] duration control
  (set `self.duration` (- (`self.duration`) DeltaSeconds))
  ;[1 1 1] core spawn control
  (if (< (`self.duration`) 0.9)
    (`ParticleSystemComponent.SetFloatParameter` (`self.FX`) "core" 0.0)
    ;[1 1 1] control end effect spawn
    (if (and (< (`self.duration`) 0.1) (not (`self.isEnd`)))
      ;[1 1 1] spawn end effect
      (set `self.isEnd` true)
      (bind _returnvalue (`GameplayStatics.SpawnEmitterAtLocation` "/Game/VFX/AdvancedMagicFX20/Particles/P_ky_warpEnd.P_ky_warpEnd" (`SceneComponent.K2_GetComponentLocation` _defaultsceneroot) (struct) (`SceneComponent.K2_GetComponentScale` _defaultsceneroot)))
      (`ParticleSystemComponent.SetVectorParameter` _returnvalue "color" (`KismetMathLibrary.Conv_LinearColorToVector` (`self.color`))))))

(event `self.ReceiveActorBeginOverlap`
  (params (OtherActor :type "Actor Object Reference")))

(fn `UserConstructionScript`
  ;[1 1 1] color control
  (`ParticleSystemComponent.SetVectorParameter` (`self.FX`) "color" (`KismetMathLibrary.Conv_LinearColorToVector` (`self.color`))))